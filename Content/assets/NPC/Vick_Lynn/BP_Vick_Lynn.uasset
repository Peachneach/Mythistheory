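; BP_Vick_Lynn is the NPC Vick Lynn, who shows dialogue lines one at a time through its Talk1 event.
; Each call increments TalkIndex, creates the WBP_Dialogue widget if none is valid, sets that line as its text and plays the Vick_Lynn sound.
; Past the last line it removes the widget and resets TalkIndex to 0, so the following call shows the line at index 1.
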(event EventTalk1
  (Math|Integer|IncrementInt (Variables|Default|GetTalkIndex)
    (:%20%20
      (if (< (Variables|Default|GetTalkIndex) (Utilities|Array|Length (Variables|Default|GetDialogue)))
        (Variables|Default|GetUI
          (:then
            _)
          (:else
            (bind _returnvalue (UserInterface|CreateWidget "/Game/assets/NPC/Vick_Lynn/WBP_Dialogue.WBP_Dialogue_C" (Game|GetPlayerController 0)))
            (bind _output_get (Variables|Default|SetUI _returnvalue))
            (UserInterface|Viewport|AddtoViewport _output_get 0)))
        (Rendering|Components|TextRender|SetText (Variables|/Game/assets/NPC/Vick_Lynn/WBP_Dialogue.WBP_Dialogue_C|GetTalkText (Variables|Default|GetUI)) (Utilities|Text|ToText(String) (Utilities|Array|Get(acopy) (Variables|Default|GetDialogue) (Variables|Default|GetTalkIndex))))
        (Audio|PlaySound2D "/Game/assets/NPC/Vick_Lynn/Vick_Lynn.Vick_Lynn" 1.0 1.0 0.0 0 0)
        (else
          (Variables|Default|SetTalkIndex 0)
          (Widget|RemovefromParent (Variables|Default|GetUI))
          (Variables|Default|SetUI 0))))))

(fn ConstructionScript)
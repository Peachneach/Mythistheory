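; BP_Pigs is a drifting sprite actor, with cloud-named parts, that loops from its start location toward Cloud1EndPosition.
; The construction script picks a random sprite and speed.
; Tick moves the actor along the normalized direction, snapping it back to the start once accumulated distance exceeds the path length.
; A timeline started at a random time adds vertical offsets to the sprite, desynchronizing instances.
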(event EventBeginPlay
  (Variables|Default|SetCloud1StartPosition (Transformation|GetActorLocation))
  (Variables|Default|SetCloud1IsMoving true)
  (Variables|Default|SetMaxDistance (Math|Vector|VectorLength (- (Variables|Default|GetCloud1EndPosition) (Variables|Default|GetCloud1StartPosition))))
  (bind _output_get (Variables|Default|SetNewVar (- (Variables|Default|GetCloud1EndPosition) (Variables|Default|GetCloud1StartPosition))))
  (Class|KismetMathLibrary|VectorNormalize _output_get 0.0)
  (Variables|Default|SetCurrentDistance 0.0)
  (Utilities|FlowControl|Sequence
    (:then_0
      (bind _newtrack_0 (Timeline|Timeline SetNewTime)
        (:Update
          (Transformation|AddRelativeLocation (Variables|Default|GetClouds_2_Sprite_0) (* "0.000000,0.000000,1.000000" (* _newtrack_0 5.0)) false false))))
    (:then_1
      (Timeline|Timeline Play))))

(event EventTick
  (params (DeltaSeconds :type Float%20%28single-precision%29))
  (bind _returnvalue (Utilities|Time|GetWorldDeltaSeconds))
  (bind _cloud1speed (Variables|Default|GetCloud1Speed))
  (bind _newvar (Variables|Default|GetNewVar))
  (bind _returnvalue_2 (* _newvar _cloud1speed _returnvalue))
  (Variables|Default|SetCurrentDistance (+ (Variables|Default|GetCurrentDistance) (Math|Vector|VectorLength _returnvalue_2)))
  (Transformation|SetActorLocation (+ (Transformation|GetActorLocation) _returnvalue_2) false false)
  (if (> (Variables|Default|GetCurrentDistance) (Variables|Default|GetMaxDistance))
    (Transformation|SetActorLocation (Variables|Default|GetCloud1StartPosition) false false)
    (Variables|Default|SetCurrentDistance 0.0)))

(fn ConstructionScript
  (Variables|Default|SetCloud1StartPosition (Transformation|GetActorLocation))
  (Rendering|Components|Sprite|SetSprite (Variables|Default|GetClouds_2_Sprite_0) (.OutItem (Utilities|Array|Random (Variables|Default|GetNew%20Sprite))))
  (Variables|Default|SetCloud1Speed (Math|Random|RandomFloatinRange 1e+02 3e+02)))